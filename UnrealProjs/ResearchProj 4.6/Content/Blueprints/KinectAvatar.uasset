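; Kinect-driven avatar actor that becomes the player's view target and mirrors the centered tracked body on a poseable mesh.
; Each tick it pins the camera to the mesh's head bone and resets HMD position, leaving positional movement to Kinect.
; While a body is tracked, its pitch-adjusted spine-base joint offsets the root horizontally from the construction-time origin, keeping height fixed.
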(event EventBeginPlay
  (bind _returnvalue (AddComponent|AddKinectInterfaceComponent false))
  (Variables|Default|SetKC _returnvalue)
  (Game|Player|SetViewTargetwithBlend (Game|GetPlayerController 0) self 0.0 "VTBlend_Linear" 0.0 false))

(event EventTick
  (params (DeltaSeconds :type Float%20%28single-precision%29))
  (bind (_centeredbody _istracked) (Class|KinectInterfaceComponent|GetCenteredBody (Variables|Default|GetKC)))
  (bind _returnvalue (Class|PoseableMeshComponent|GetBoneLocationbyName (Variables|Default|GetKinectPoseableMesh1) "head" "ComponentSpace"))
  (Transformation|SetRelativeLocation (Variables|Default|GetAvatarCamera) _returnvalue false)
  (Class|HeadMountedDisplayFunctionLibrary|ResetOrientationandPosition 0.0 "Position")
  (if _istracked
    (CallFunction|MoveRootPositionwithBody _centeredbody)
    (bind _centeredbody_2 (Class|KinectInterfaceComponent|GetCenteredBody (Variables|Default|GetKC)))
    (Variables|/Script/Kinect4Unreal.KinectPoseableMeshComponent|SetTargetBody (Variables|Default|GetKinectPoseableMesh1) _centeredbody_2)))

(fn ConstructionScript
  (Variables|Default|SetmeshHeight (.Y (Math|Vector|BreakVector (.BoxExtent (Collision|GetComponentBounds (Variables|Default|GetKinectPoseableMesh1))))))
  (Variables|Default|SetactorFloorOrigin (Transformation|GetActorLocation)))

(fn MoveRootPositionwithBody
  (params (BodyNumber :type EBodyNumber%20Enum))
  (bind _actorfloororigin (Variables|Default|GetactorFloorOrigin))
  (bind _returnvalue (Class|KinectInterfaceComponent|GetPitchAdjustedJointPosition (Variables|Default|GetKC) "SpineBase" BodyNumber))
  (Transformation|SetRelativeLocation (VehicleSound|GetRootComponent) (Math|Vector|MakeVector (.X (Math|Vector|BreakVector (+ _actorfloororigin _returnvalue))) (.Y (Math|Vector|BreakVector (+ _actorfloororigin _returnvalue))) (.Z (Math|Vector|BreakVector _actorfloororigin))) false))