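; TagPrism runs a timed target-tagging experiment, placing the player at its center and turning the TagBoxes from its upper and lower containers inward.
; Space and Enter start experiments 1 and 2, each with a fixed random seed for a repeatable target order.
; Each hit records seconds since the start and readies a different random box.
; At the goal count, times are saved comma-separated to a hard-coded local folder.
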(event Custom|ChildInteractedWith
  (params (Sender :type Tag%20Box%20Object%20Reference))
  (bind _experimentstart (Variables|Default|GetexperimentStart))
  (bind _seconds (Class|VictoryBPFunctionLibrary|RealWorldTimeGetTimePassedSincePreviousTime _experimentstart))
  (switch int (Variables|Default|GetexperimentID)
    (:1
      (Utilities|Array|Add (Variables|Default|Getexperiement1Hits) _seconds))
    (:2
      (Utilities|Array|Add (Variables|Default|Getexperiement2Hits) _seconds)))
  (Utilities|IncrementTargetsHit)
  (if (>= (Variables|Default|GettargetsHit) (Variables|Default|GetgoalTargetsHit))
    (CallFunction|StopTestandSaveResults)
    (else
      (bind _item (CallFunction|GetPredictableRandChild Sender (Variables|Default|GettagBoxes)))
      (Default|SetPrismReadyto _item true))))

(event EventBeginPlay
  (bind _returnvalue (Transformation|GetActorLocation))
  (bind _returnvalue_2 (+ _returnvalue "0, 0,90.000000"))
  (Transformation|SetActorLocation (Game|GetPlayerController 0) _returnvalue_2 false)
  (Transformation|SetActorLocation (Game|Player|GetPlayerPawn 0) _returnvalue_2 false)
  (for _array_element (Variables|Default|GettagBoxes)
    (EventDispatchers|BindEventtoInteractedEvent _array_element (delegate Custom|ChildInteractedWith))
    (Input|EnableInput (Game|GetPlayerController 0))
    (Transformation|SetActorRotation _array_element (Math|Rotator|FindLookatRotation (Transformation|GetActorLocation _array_element) (+ _returnvalue_2 "0, 0,40.000000")))))

(event Input|KeyboardEvents|SpaceBar
  (:Pressed
    (Variables|Default|SetexperimentID 1)
    (Math|Random|SetRandomStreamSeed (Variables|Default|GetrandStream) 2)
    (Variables|Default|SetexperimentStart (.ReturnValue (Class|VictoryBPFunctionLibrary|RealWorldTimeGetCurrentOSTime)))
    (bind _item (CallFunction|GetPredictableRandChild 0 (Variables|Default|GettagBoxes)))
    (Default|SetPrismReadyto _item true)
    (Variables|Default|SettargetsHit 0)))

(event Input|KeyboardEvents|Enter
  (:Pressed
    (Variables|Default|SetexperimentID 2)
    (Math|Random|SetRandomStreamSeed (Variables|Default|GetrandStream) 0)
    (Variables|Default|SetexperimentStart (.ReturnValue (Class|VictoryBPFunctionLibrary|RealWorldTimeGetCurrentOSTime)))
    (bind _item (CallFunction|GetPredictableRandChild 0 (Variables|Default|GettagBoxes)))
    (Default|SetPrismReadyto _item true)
    (Variables|Default|SettargetsHit 0)))

(fn ConstructionScript
  (Utilities|GetTagBoxesfromParent (Variables|Default|GetLowerContainer)
    (:Out
      (Utilities|GetTagBoxesfromParent (Variables|Default|GetUpperContainer)))))

(fn StopTestandSaveResults
  (switch int (Variables|Default|GetexperimentID)
    (:1
      (LocalVariables|SetvaluesToSave (Variables|Default|Getexperiement1Hits)))
    (:2
      (LocalVariables|SetvaluesToSave (Variables|Default|Getexperiement2Hits))))
  (for _array_element (LocalVariables|GetvaluesToSave)
    (LocalVariables|SethitString (Utilities|String|Append (LocalVariables|GethitString) (Utilities|String|Append (Utilities|String|ToString(Float) _array_element) ", "))))
  (LocalVariables|SethitString (Utilities|String|LeftChop (LocalVariables|GethitString) 2))
  (bind _returnvalue (Class|VictoryBPFunctionLibrary|FileIOSaveStringTexttoFile "J:\\Users\\Peter\\SkyDrive\\Documents\\CSC 4001\\ExperimentResults\\Tag" (Utilities|String|Append (Variables|Default|GetexperimentStart) ".txt") (LocalVariables|GethitString) false))
  (Development|PrintString "Saving....")
  (Development|PrintString (Utilities|String|ToString(Boolean) _returnvalue)))

(fn GetPredictableRandChild
  (params (exception :type Tag%20Box%20Object%20Reference) (TargetArray :type Array%20of%20Tag%20Box%20Object%20References))
  (LocalVariables|SetrandTagBox (Utilities|Array|Get(acopy) TargetArray (Math|Random|RandomIntegerinRangefromStream 0 (- (Utilities|Array|Length TargetArray) 1) (Variables|Default|GetrandStream))))
  (if (== (LocalVariables|GetrandTagBox) exception)
    (bind _item (CallFunction|GetPredictableRandChild exception TargetArray))
    (LocalVariables|Setoutput _item)
    (else
      (LocalVariables|Setoutput (LocalVariables|GetrandTagBox))))
  (return (LocalVariables|Getoutput)))