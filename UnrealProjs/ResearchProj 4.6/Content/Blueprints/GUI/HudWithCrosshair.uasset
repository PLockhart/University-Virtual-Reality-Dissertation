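; HUD Blueprint that draws a simple crosshair at the center of the screen.
; Each DrawHUD event computes the screen midpoint from the viewport size and draws a horizontal and a vertical line through it in a fixed blue color.
; The CrosshairLength variable sets how far each line extends either side of the center.
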(event EventDrawHUD
  (params (SizeX :type Integer) (SizeY :type Integer))
  (bind _returnvalue (Math|Conversions|ToFloat(Integer) SizeX))
  (bind _returnvalue_2 (Math|Conversions|ToFloat(Integer) SizeY))
  (bind _crosshairlength (Variables|Default|GetcrosshairLength))
  (bind _returnvalue_3 (/ _returnvalue_2 2.0))
  (bind _returnvalue_4 (/ _returnvalue 2.0))
  (Class|HUD|DrawLine (- _returnvalue_4 _crosshairlength) _returnvalue_3 (+ _returnvalue_4 _crosshairlength) _returnvalue_3 "(R=0.041662,G=0.009275,B=0.575000,A=1.000000)")
  (Class|HUD|DrawLine _returnvalue_4 (- _returnvalue_3 _crosshairlength) _returnvalue_4 (+ _returnvalue_3 _crosshairlength) "(R=0.041662,G=0.009275,B=0.575000,A=1.000000)"))

(fn ConstructionScript)