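; Kinect-driven radial menu HUD, opened when the centered body's left hand is closed at the start and end of a delay (or by debug key B).
; The right hand's neck-relative position, unrotated by neck orientation, is compared to its position at opening to form a 2D offset.
; Beyond a minimum length, that offset's angle selects one of four items in cardinal sectors.
; DrawHUD draws the offset from screen center.
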(event Custom|OnOpenGesture_Event
  (bind _kc (Variables|Default|GetKC))
  (if (not (Variables|Default|GetisDelayedWaitingForGesture))
    (Variables|Default|SetisDelayedWaitingForGesture true)
    (Utilities|FlowControl|Delay (Variables|Default|GetopenGestureDuration))
    (bind _centeredbody (Class|KinectInterfaceComponent|GetCenteredBody _kc))
    (bind _returnvalue (CallFunction|IsOpenGesturePerformed _kc _centeredbody))
    (if _returnvalue
      (bind _returnvalue_2 (CallFunction|GetRotatedRelativeInteractingJointPosition _centeredbody))
      (CallFunction|ActivateGUI _returnvalue_2))
    (Variables|Default|SetisDelayedWaitingForGesture false)))

(event EventBeginPlay
  (|CallParentFunction)
  (CallFunction|InitKinectResearchRadial))

(event EventTick
  (params (DeltaSeconds :type Float%20%28single-precision%29))
  (bind _selectionangle (Variables|Default|GetselectionAngle))
  (|CallParentFunction DeltaSeconds)
  (bind _centeredbody (Class|KinectInterfaceComponent|GetCenteredBody (Variables|Default|GetKC)))
  (bind _returnvalue (Class|RadialHUD|IsRadialActive))
  (if _returnvalue
    (CallFunction|CalculateRadialOffset2D _centeredbody)
    (Math|Float|CompareFloat (Math|Vector2D|Vector2DLength (Variables|Default|Get2dRadialOffset)) (Variables|Default|GetminOffsetForSelection)
      (:>
        (CallFunction|CalculateSelectionAngle)
        (bind _liesbetween (CallFunction|IsFloatBetweenFloats _selectionangle 3.4e+02 3.6e+02))
        (bind _liesbetween_2 (CallFunction|IsFloatBetweenFloats _selectionangle 0.0 2e+01))
        (if (or _liesbetween _liesbetween_2)
          (Class|RadialHUD|SelectRadialItem (Utilities|GetRadialItem))
          (else
            (bind _liesbetween_3 (CallFunction|IsFloatBetweenFloats _selectionangle 7e+01 1.1e+02))
            (if _liesbetween_3
              (Class|RadialHUD|SelectRadialItem (Utilities|GetRadialItem 1))
              (else
                (bind _liesbetween_4 (CallFunction|IsFloatBetweenFloats _selectionangle 1.6e+02 2e+02))
                (if _liesbetween_4
                  (Class|RadialHUD|SelectRadialItem (Utilities|GetRadialItem 2))
                  (else
                    (bind _liesbetween_5 (CallFunction|IsFloatBetweenFloats _selectionangle 2.5e+02 2.9e+02))
                    (if _liesbetween_5
                      (Class|RadialHUD|SelectRadialItem (Utilities|GetRadialItem 3)))))))))))
    (else
      (CallFunction|ActivateGUIonGesture _centeredbody))))

(event EventSetRadialGUIWidgetVisbility
  (params (isVisible :type Boolean))
  (bind _radialhud (Variables|Default|GetRadialHUD))
  (if isVisible
    (Widget|SetVisibility _radialhud "Visible")
    (else
      (Widget|SetVisibility _radialhud "Hidden"))))

(event EventAssignWidgetsforItems
  (params (items :type Array%20of%20Radial%20Item%20Structures))
  (for _array_element (Variables|/Game/Blueprints/GUI/RadialMenu.RadialMenu_C|GetRadialButtons (Variables|Default|GetRadialHUD))
    (Widget|SetVisibility _array_element "Hidden"))
  (for (_array_element_2 _array_index) items
    (CallFunction|SetupWidgetforRadialItem _array_element_2 _array_index)))

(event EventDrawHUD
  (params (SizeX :type Integer) (SizeY :type Integer))
  (bind _returnvalue (Math|Conversions|ToFloat(Integer) SizeX))
  (bind _returnvalue_2 (Math|Conversions|ToFloat(Integer) SizeY))
  (bind _2dradialoffset (Variables|Default|Get2dRadialOffset))
  (bind _returnvalue_3 (/ _returnvalue_2 2.0))
  (bind _returnvalue_4 (/ _returnvalue 2.0))
  (bind _returnvalue_5 (Math|Vector2D|MakeVector2D _returnvalue_4 _returnvalue_3))
  (bind _returnvalue_6 (+ _returnvalue_5 _2dradialoffset))
  (bind (_x _y) (Math|Vector2D|BreakVector2D _returnvalue_6))
  (|CallParentFunction SizeX SizeY)
  (bind _returnvalue_7 (Class|RadialHUD|IsRadialActive))
  (if _returnvalue_7
    (Class|HUD|DrawLine _returnvalue_4 _returnvalue_3 _x _y "(R=0.890000,G=0.053731,B=0.286482,A=1.000000)")))

(event Input|KeyboardEvents|B
  ;[1 1 1] Debugging purposes for starting GUI
  (:Pressed
    (CallFunction|ActivateGUI "0, 0, 0")))

(fn ConstructionScript)

(fn SpawnRadialHud
  (bind _returnvalue (UserInterface|CreateWidget "/Game/Blueprints/GUI/RadialMenu.RadialMenu_C"))
  (Variables|Default|SetRadialHUD _returnvalue)
  (UserInterface|Viewport|AddtoViewport (Variables|Default|GetRadialHUD))
  (Widget|SetVisibility (Variables|Default|GetRadialHUD) "Hidden")
  (return))

(fn ActivateGUIonGesture
  (params (BodyNumber :type EBodyNumber%20Enum :default "Body0"))
  (bind _returnvalue (CallFunction|IsOpenGesturePerformed (Variables|Default|GetKC) BodyNumber))
  (if _returnvalue
    (CallFunction|OnOpenGestureEvent)))

(fn GetRadialButtonatIndex
  (params (Index :type Integer))
  (return (Utilities|Array|Get(acopy) (Variables|/Game/Blueprints/GUI/RadialMenu.RadialMenu_C|GetRadialButtons (Variables|Default|GetRadialHUD)) Index)))

(fn SetWidgetProperties
  (params (buttonText :type Text%20Block%20Object%20Reference) (widget :type Widget%20Object%20Reference) (theItem :type Radial%20Item%20Structure))
  (bind (_displayname _isempty) (Class|RadialHUD|GetRadialItemData theItem))
  (Rendering|Components|TextRender|SetText buttonText (Utilities|Text|ToText(String) _displayname))
  (if _isempty
    _
    (else
      (Widget|SetVisibility widget "Visible")))
  (return))

(fn SetupWidgetforRadialItem
  (params (Item :type Radial%20Item%20Structure) (Index :type Integer))
  (bind _item (CallFunction|GetRadialButtonatIndex Index))
  (Variables|/Game/Blueprints/GUI/RadialWidget.RadialWidget_C|SetItem _item Item)
  (CallFunction|SetWidgetProperties (Variables|/Game/Blueprints/GUI/RadialWidget.RadialWidget_C|GetButtonText _item) _item Item))

(fn ActivateGUI
  (params (originPosition :type Vector))
  (Class|RadialHUD|RevealHUD)
  (Class|RadialHUD|StartInteracting originPosition))

(fn ConvertKinectVectorto2DVector
  (params (InVec :type Vector))
  (bind (_x _y _z) (Math|Vector|BreakVector InVec))
  (return (Math|Vector2D|MakeVector2D (* -1 _y) _z)))

(fn InitKinectResearchRadial
  (Variables|Default|SetInteractingRefJoint "Neck")
  (Variables|Default|SetInteractingJoint "HandRight")
  (CallFunction|SpawnRadialHud)
  (bind _returnvalue (AddComponent|AddKinectInterfaceComponent false))
  (Variables|Default|SetKC _returnvalue)
  (return))

(fn GetRotatedRelativeInteractingJointPosition
  (params (BodyNumber :type EBodyNumber%20Enum :default "Body0"))
  (bind _returnvalue (Class|KinectInterfaceComponent|GetJointRelativePosition (Variables|Default|GetKC) (Variables|Default|GetInteractingRefJoint) BodyNumber (Variables|Default|GetInteractingJoint) BodyNumber))
  (bind _returnvalue_2 (CallFunction|RotateVectorAroundInteractingReferenceJoint _returnvalue BodyNumber))
  (return _returnvalue_2))

(fn RotateVectorAroundInteractingReferenceJoint
  (params (A :type Vector) (BodyNumber :type EBodyNumber%20Enum :default "Body0"))
  (bind _returnvalue (Class|KinectInterfaceComponent|GetSmoothedJointOrientation (Variables|Default|GetKC) (Variables|Default|GetInteractingRefJoint) BodyNumber))
  (return (Math|Vector|UnrotateVector A _returnvalue)))

(fn CalculateRadialOffset2D
  (params (BodyNumber :type EBodyNumber%20Enum))
  (bind _returnvalue (CallFunction|GetRotatedRelativeInteractingJointPosition BodyNumber))
  (bind _returnvalue_2 (Class|RadialHUD|GetOriginPosition))
  (bind _returnvalue_3 (CallFunction|ConvertKinectVectorto2DVector (- _returnvalue_2 _returnvalue)))
  (Variables|Default|Set2dRadialOffset _returnvalue_3)
  (return))

(fn IsFloatBetweenFloats
  (params (input :type Float%20%28single-precision%29) (lowerBound :type Float%20%28single-precision%29) (upperBound :type Float%20%28single-precision%29))
  (return (and (>= input lowerBound) (<= input upperBound))))

(fn CalculateSelectionAngle
  (bind _2dradialoffset (Variables|Default|Get2dRadialOffset))
  (bind (_x _y) (Math|Vector2D|BreakVector2D _2dradialoffset))
  (bind _returnvalue (Class|KismetMathLibrary|DegAtan2 _y _x))
  (bind _returnvalue_2 (+ _returnvalue 9e+01))
  (Math|Float|CompareFloat _returnvalue_2 0.0
    (:>
      (Variables|Default|SetselectionAngle _returnvalue_2 :!label _label))
    (:==
      (goto _label))
    (:<
      (Variables|Default|SetselectionAngle (+ _returnvalue_2 3.6e+02))))
  (return))

(fn IsOpenGesturePerformed
  (params (self2 :type Kinect%20Interface%20Component%20Object%20Reference) (BodyNumber :type EBodyNumber%20Enum :default "Body0"))
  (bind _returnvalue (Class|KinectInterfaceComponent|GetHandState self2 "Left" BodyNumber))
  (bind _returnvalue_2 (Class|KinectInterfaceComponent|GetHandState self2 "Left" BodyNumber))
  (return (and (Utilities|Enum|Equal(Enum) _returnvalue_2 "Closed") (Utilities|Enum|Equal(Enum) _returnvalue "Closed"))))