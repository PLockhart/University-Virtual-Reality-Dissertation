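; Fireworks launcher actor that fires BP_Fireworks_Shell actors from its arrow component whenever LaunchShell is called.
; Each shell spawns with random angular spread, a randomly picked burst particle system and a random burst count, inheriting the launcher's velocity, rotation, lifetime and timing ranges.
; A launch plays a sound and fires a spawned dispatcher, and the launcher relays the shell's explosion through its own exploded dispatcher.
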(event Custom|LaunchShell
  (bind _arrow1 (Variables|Default|GetArrow1))
  (bind _burstparticlesystems (Variables|BurstProperties|GetBurstParticleSystems))
  (bind _returnvalue (Transformation|GetWorldTransform _arrow1))
  (bind (_location _rotation) (Math|Transform|BreakTransform _returnvalue))
  (bind _returnvalue_2 (Game|SpawnActorfromClass "/Game/Fireworks/BP_Fireworks_Shell.BP_Fireworks_Shell_C" (Math|Transform|MakeTransform _location (Math|Rotator|CombineRotators _rotation (Class|KismetMathLibrary|MakeRot (Math|Random|RandomFloatinRange (* (Variables|Default|GetRandomAngle) -1.0) (Variables|Default|GetRandomAngle)) (Math|Random|RandomFloatinRange (* (Variables|Default|GetRandomAngle) -1.0) (Variables|Default|GetRandomAngle)) (Math|Random|RandomFloatinRange (* (Variables|Default|GetRandomAngle) -1.0) (Variables|Default|GetRandomAngle))))) true (Variables|ShellProperties|GetMaxRotationSpeed) (Variables|ShellProperties|GetMinRotationSpeed) (Variables|ShellProperties|GetMaxLaunchVelocity) (Variables|ShellProperties|GetMinLaunchVelocity) (Variables|ShellProperties|GetShellMaxLife) (Variables|ShellProperties|GetShellminLife) (Variables|BurstProperties|GetMaxBurstTime) (Variables|BurstProperties|GetMinBurstTime) (Utilities|Array|Get(acopy) _burstparticlesystems (Math|Random|RandomInteger (Utilities|Array|Length _burstparticlesystems))) (Variables|ShellProperties|GetShellParticleSystem) false (Math|Random|RandomIntegerinRange 1 (Variables|BurstProperties|GetMaxNumberOfBursts)) (Variables|BurstProperties|GetSecondaryBurstDelay)))
  (Audio|PlaySoundatLocation "/Game/Audio/Fireworks/firework_rocket_launch.firework_rocket_launch" _location)
  (Default|CallFireworkSpawnedEvent)
  (EventDispatchers|BindEventtoFireworkExplodedEvent _returnvalue_2 (delegate Custom|FireworkExplodedEvent_Event)))

(event Custom|FireworkExplodedEvent_Event
  (Default|CallFireworkExplodedEvent))

(fn ConstructionScript)