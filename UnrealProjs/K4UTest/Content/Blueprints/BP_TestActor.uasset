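; BP_TestActor is a test actor that mirrors a Kinect-tracked player's hands with two meshes.
; BeginPlay caches player controller 0 as a KinectPlayerController.
; Each Tick finds the centered body and copies its left and right hand joint absolute positions into the relative locations of the matching hand meshes, without sweep.
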(event EventBeginPlay
  (bind _askinectplayercontroller (Utilities|Casting|CastToKinectPlayerController (Game|GetPlayerController 0)))
  (Variables|Default|SetKPC _askinectplayercontroller))

(event EventTick
  (params (DeltaSeconds :type Float%20%28single-precision%29))
  (bind _centeredbody (Class|KinectPlayerController|GetCenteredBody (Variables|Default|GetKPC)))
  (bind _returnvalue (Class|KinectPlayerController|GetJointAbsolutePosition (Variables|Default|GetKPC) "HandLeft" _centeredbody))
  (Transformation|SetRelativeLocation (Variables|Default|GetLeftHandmesh) _returnvalue false)
  (bind _returnvalue_2 (Class|KinectPlayerController|GetJointAbsolutePosition (Variables|Default|GetKPC) "HandRight" _centeredbody))
  (Transformation|SetRelativeLocation (Variables|Default|GetRightHandMesh) _returnvalue_2 false))

(fn ConstructionScript)