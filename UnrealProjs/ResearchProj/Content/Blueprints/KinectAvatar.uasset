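; Kinect-driven avatar actor that follows the body the Kinect reports as centered and serves as the player's view target.
; On BeginPlay it caches the KinectPlayerController and switches the view to itself.
; Each tick it sets its root location to that body's head joint, offset along Y by the poseable mesh's bounds extent.
; It also retargets the KinectPoseableMesh to the centered body every frame.
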(event EventBeginPlay
  (bind _askinectplayercontroller (Utilities|Casting|CastToKinectPlayerController (Game|GetPlayerController 0)))
  (Variables|Default|SetKPC _askinectplayercontroller)
  (Game|Player|SetViewTargetwithBlend (Game|GetPlayerController 0) self 0.0 "VTBlend_Linear" 0.0 false))

(event EventTick
  (params (DeltaSeconds :type Float%20%28single-precision%29))
  (bind _centeredbody (Class|KinectPlayerController|GetCenteredBody (Variables|Default|GetKPC)))
  (bind _returnvalue (Class|KinectPlayerController|GetJointAbsolutePosition (Variables|Default|GetKPC) "Head" _centeredbody))
  (Transformation|SetRelativeLocation (VehicleSound|GetRootComponent) (+ _returnvalue (Math|Vector|MakeVector 0.0 (.Y (Math|Vector|BreakVector (.BoxExtent (Collision|GetComponentBounds (Variables|Default|GetKinectPoseableMesh1))))) 0.0)) false)
  (bind _centeredbody_2 (Class|KinectPlayerController|GetCenteredBody (Variables|Default|GetKPC)))
  (Variables|/Script/Kinect4Unreal.KinectPoseableMeshComponent|SetTargetBody (Variables|Default|GetKinectPoseableMesh1) _centeredbody_2))

(fn ConstructionScript)